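; Time stop actor that pauses the whole game for a set duration, then resumes it automatically.
; The PauseMe event records the unpaused world time and pauses the game.
; While the game is paused, Tick compares unpaused time against that timestamp and unpauses once PauseDurationSec has elapsed.
; Tick checks only the global pause state, so it does not distinguish pauses started elsewhere.
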(event Custom|PauseMe
  (Variables|Default|SetPauseTime (Class|GameplayStatics|GetUnpausedTimeSeconds))
  (Game|SetGamePaused true))

(event EventTick
  (params (DeltaSeconds :type Float%20%28single-precision%29))
  (if (Game|IsGamePaused)
    (if (>= (- (Class|GameplayStatics|GetUnpausedTimeSeconds) (Variables|Default|GetPauseTime)) (Variables|Default|GetPauseDurationSec))
      (Game|SetGamePaused false))))

(fn ConstructionScript)